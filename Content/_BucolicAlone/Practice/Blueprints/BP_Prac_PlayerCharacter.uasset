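; Practice player character with Enhanced Input movement, a quick-slot inventory, health and equippable hat and weapon meshes.
; Mouse wheel selects a HUD slot; left click consumes, equips or reads its item by type.
; Pickups replace the selected slot, spawning the old item at the throw point.
; Being hit by an actor triggers a timed ragdoll knockdown with impulse, then reattaches the mesh to the capsule and restores walking.
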(event `CreateMainHUD`
  ;[1 1 1] Create Main Widget HUD
  (bind _returnvalue (`|CreateWidget` "/Game/_BucolicAlone/Practice/PracticeBP/06_InventorySystem/Widget/WBP_MainWidgetHUD.WBP_MainWidgetHUD_C" (`GameplayStatics.GetPlayerController` 0)))
  (`UserWidget.AddToViewport` _returnvalue 0)
  (set `self.WidgetReference` _returnvalue))

(event `self.ReceiveBeginPlay`
  ;[1 1 1] Add mapping context
  (`|ExecutionSequence`
    (:`then_0`
      (bind `_as플레이어_컨트롤러` (cast `PlayerController` (`self.GetController`)))
      (bind _returnvalue (pcsubsystem `EnhancedInputLocalPlayerSubsystem` `_as플레이어_컨트롤러`))
      (`/Engine/EditorBlueprintResources/StandardMacros.IsValid` _returnvalue
        (:`Is Valid`
          (`EnhancedInputSubsystemInterface.AddMappingContext` _returnvalue "/Game/_BucolicAlone/Practice/Inputs/IMC_Prac_Default.IMC_Prac_Default" 0 (struct)))))
    (:`then_1`
      (`self.CreateMainHUD`))))

(event `EquipHat`
  (params (NewMesh :type "StaticMesh Object Reference"))
  ;[1 1 1] 02_EquipHatEvent
  (`StaticMeshComponent.SetStaticMesh` (`self.HatMesh`) NewMesh)
  (`SceneComponent.K2_AttachToComponent` (`self.HatMesh`) (`self.Mesh`) "hatSocket" "KeepRelative" "KeepRelative" "KeepRelative" true))

(event `PickUpItemEvent`
  (params (ItemInfo :type "/Game/_BucolicAlone/Practice/PracticeBP/06_InventorySystem/Data/Structures/S_ItemStructure Structure"))
  ;[1 1 1] Item Pickup
  (`self.AddItem` ItemInfo))

(event `CreateHealthBar`
  ;[1 1 1] 03_DamageBox
  (bind _returnvalue (`|CreateWidget` "/Game/_BucolicAlone/Practice/PracticeBP/03_DamageBox/Blueprints/WBP_HealthBar.WBP_HealthBar_C" (`GameplayStatics.GetPlayerController` 0)))
  (`UserWidget.AddToViewport` _returnvalue 0))

(event `Key|MouseScrollDown`
  (params (Key :type "Key Structure"))
  ;[1 1 1] Item Select
  (:`Pressed`
    (if (not (== (`self.SelectedIndex`) (`self.MaxInventoryIndex`)))
      (bind _result (`/Engine/EditorBlueprintResources/StandardMacros.IncrementInt` (`self.SelectedIndex`))
        (:`  `
          (`/Game/_BucolicAlone/Practice/PracticeBP/06_InventorySystem/Widget/WBP_MainWidgetHUD.SelectItem` (`self.WidgetReference`) _result))))))

(event `EnhancedInput|/Game/_BucolicAlone/Practice/Inputs/Actions/IA_Prac_Look`
  (params (ActionValue :type "Vector2D Structure") (ElapsedSeconds :type "Float (double-precision)") (TriggeredSeconds :type "Float (double-precision)") (InputAction :type "InputAction Object Reference" :default "/Game/_BucolicAlone/Practice/Inputs/Actions/IA_Prac_Look.IA_Prac_Look"))
  ;[1 1 1] IA_Prac_Look
  (:`Triggered`
    (`self.AddControllerYawInput` ActionValue_X)
    (`self.AddControllerPitchInput` (* ActionValue_Y -1.0))))

(event `EnhancedInput|/Game/_BucolicAlone/Practice/Inputs/Actions/IA_Prac_Jump`
  (params (ActionValue :type Boolean) (ElapsedSeconds :type "Float (double-precision)") (TriggeredSeconds :type "Float (double-precision)") (InputAction :type "InputAction Object Reference" :default "/Game/_BucolicAlone/Practice/Inputs/Actions/IA_Prac_Jump.IA_Prac_Jump"))
  ;[1 1 1] IA_Prac_Jump
  (:`Started`
    (`self.Jump`))
  (:`Completed`
    (`self.StopJumping`)))

(event `self.ReceiveAnyDamage`
  (params (Damage :type "Float (single-precision)") (DamageType :type "DamageType Object Reference") (InstigatedBy :type "Controller Object Reference") (DamageCauser :type "Actor Object Reference"))
  ;[1 1 1] 03_DamageBox
  (set `self.Health` (- (`self.Health`) Damage)))

(event `Key|MouseScrollUp`
  (params (Key :type "Key Structure"))
  ;[1 1 1] Item Select
  (:`Pressed`
    (if (not (== (`self.SelectedIndex`) 0))
      (bind _result (`/Engine/EditorBlueprintResources/StandardMacros.DecrementInt` (`self.SelectedIndex`))
        (:`  `
          (`/Game/_BucolicAlone/Practice/PracticeBP/06_InventorySystem/Widget/WBP_MainWidgetHUD.SelectItem` (`self.WidgetReference`) _result))))))

(event `EnhancedInput|/Game/_BucolicAlone/Practice/Inputs/Actions/IA_Prac_Move`
  (params (ActionValue :type "Vector2D Structure") (ElapsedSeconds :type "Float (double-precision)") (TriggeredSeconds :type "Float (double-precision)") (InputAction :type "InputAction Object Reference" :default "/Game/_BucolicAlone/Practice/Inputs/Actions/IA_Prac_Move.IA_Prac_Move"))
  (bind (_returnvalue_roll _returnvalue_pitch _returnvalue_yaw) (`KismetMathLibrary.BreakRotator` (`self.GetControlRotation`)))
  (bind (_returnvalue_roll_2 _returnvalue_pitch_2 _returnvalue_yaw_2) (`KismetMathLibrary.BreakRotator` (`self.GetControlRotation`)))
  ;[1 1 1] IA_Prac_Move
  (:`Triggered`
    (`self.AddMovementInput` (`KismetMathLibrary.GetRightVector` (`KismetMathLibrary.MakeRotator` _returnvalue_roll 0.0 _returnvalue_yaw)) ActionValue_X)
    (`self.AddMovementInput` (`KismetMathLibrary.GetForwardVector` (`KismetMathLibrary.MakeRotator` 0.0 0.0 _returnvalue_yaw_2)) ActionValue_Y)))

(event `HitByHitActor`
  (params (HitRotation :type "Vector Structure"))
  ;[1 1 1] 05_HitActor
  (if (not (`self.IsKnockDown`))
    (set `self.IsKnockDown` true)
    (`PrimitiveComponent.SetSimulatePhysics` (`self.Mesh`) true)
    (`PrimitiveComponent.AddImpulse` (`self.Mesh`) (`KismetMathLibrary.MakeVector` (.x (* HitRotation 50000.0)) (.y (* HitRotation 50000.0)) 50000.0) "None" false)
    (`CharacterMovementComponent.DisableMovement` (`self.CharacterMovement`))
    (`KismetSystemLibrary.Delay` 3.0)
    (`PrimitiveComponent.SetSimulatePhysics` (`self.Mesh`) false)
    (`SceneComponent.K2_AttachToComponent` (`self.Mesh`) (`self.CapsuleComponent`) "None" "SnapToTarget" "SnapToTarget" "KeepRelative" true)
    (`SceneComponent.K2_SetRelativeLocation` (`self.Mesh`) (0.0 0.0 -90.0) false false)
    (`SceneComponent.K2_SetRelativeRotation` (`self.Mesh`) (struct :`Yaw` 270.0) false false)
    (`CharacterMovementComponent.SetMovementMode` (`self.CharacterMovement`) "MOVE_Walking" 0)
    (set `self.IsKnockDown` false)))

(event `Key|LeftMouseButton`
  (params (Key :type "Key Structure"))
  ;[1 1 1] Use Item
  (:`Pressed`
    (`self.UseItem` (`|GetArrayItem` (`self.InventoryArray`) (`self.SelectedIndex`)))))

(fn `AddItem`
  (params (NewItem :type "/Game/_BucolicAlone/Practice/PracticeBP/06_InventorySystem/Data/Structures/S_ItemStructure Structure (by ref)"))
  (bind _selectedindex (`self.SelectedIndex`))
  (bind (_itemtype _mesh _damage _itemname _itemicon _itemtext _itemclass) (break `/Game/_BucolicAlone/Practice/PracticeBP/06_InventorySystem/Data/Structures/S_ItemStructure` (`|GetArrayItem` (`self.InventoryArray`) (`self.SelectedIndex`))))
  (if (`KismetSystemLibrary.IsValidClass` _itemclass)
    ;[1 1 1] Deequip current equiped item
    (if (`|EnumEquality` _itemtype "NewEnumerator1")
      (`self.Deequip`))
    ;[1 1 1] Item Change
    (`|SpawnActorFromClass` _itemclass (`KismetMathLibrary.MakeTransform` (`SceneComponent.K2_GetComponentLocation` (`self.ItemThrowPoint`))) "Undefined" "MultiplyWithRoot" null null))
  ;[1 1 1] Add to Inventory Array & Update QuickSlot Image
  (`KismetArrayLibrary.Array_Set` (`self.InventoryArray`) _selectedindex NewItem)
  (`/Game/_BucolicAlone/Practice/PracticeBP/06_InventorySystem/Widget/WBP_MainWidgetHUD.UpdateImage` (`self.WidgetReference`) _selectedindex (`.ItemIcon_14_E28476C64BC14F732EBEFA8ADE055CFC` (break `/Game/_BucolicAlone/Practice/PracticeBP/06_InventorySystem/Data/Structures/S_ItemStructure` NewItem))))

(fn `ConsumeItem`
  (params (ItemInfo :type "/Game/_BucolicAlone/Practice/PracticeBP/06_InventorySystem/Data/Structures/S_ItemStructure Structure"))
  (bind _selectedindex (`self.SelectedIndex`))
  (set `self.Health` (`KismetMathLibrary.FClamp` (+ (`self.Health`) (`.Damage_10_042BBBE84312C4F8B415089226098BE8` (break `/Game/_BucolicAlone/Practice/PracticeBP/06_InventorySystem/Data/Structures/S_ItemStructure` ItemInfo))) 0.0 100.0))
  (`KismetArrayLibrary.Array_Set` (`self.InventoryArray`) _selectedindex)
  (`/Game/_BucolicAlone/Practice/PracticeBP/06_InventorySystem/Widget/WBP_MainWidgetHUD.RemoveImage` (`self.WidgetReference`) _selectedindex))

(fn `Deequip`
  (`StaticMeshComponent.SetStaticMesh` (`self.M_Weapon`) null))

(fn `EquipItem`
  (params (ItemInfo :type "/Game/_BucolicAlone/Practice/PracticeBP/06_InventorySystem/Data/Structures/S_ItemStructure Structure"))
  (`StaticMeshComponent.SetStaticMesh` (`self.M_Weapon`) (`.Mesh_8_55F63B8B4590EDFB7E1528ABF8B45CD2` (break `/Game/_BucolicAlone/Practice/PracticeBP/06_InventorySystem/Data/Structures/S_ItemStructure` ItemInfo)))
  (`SceneComponent.K2_AttachToComponent` (`self.M_Weapon`) (`self.Mesh`) "WeaponSocket" "SnapToTarget" "SnapToTarget" "SnapToTarget" true))

(fn `ReadItem`
  (params (ItemInfo :type "/Game/_BucolicAlone/Practice/PracticeBP/06_InventorySystem/Data/Structures/S_ItemStructure Structure"))
  (if (`self.IsBookOpen?`)
    (`/Game/_BucolicAlone/Practice/PracticeBP/06_InventorySystem/Widget/WBP_MainWidgetHUD.CloseBook` (`self.WidgetReference`))
    (set `self.IsBookOpen?` false)
    (else
      (`/Game/_BucolicAlone/Practice/PracticeBP/06_InventorySystem/Widget/WBP_MainWidgetHUD.OpenBook` (`self.WidgetReference`) (`.ItemText_17_D5E020604EF04B0B3AD549B0312B91C6` (break `/Game/_BucolicAlone/Practice/PracticeBP/06_InventorySystem/Data/Structures/S_ItemStructure` ItemInfo)))
      (set `self.IsBookOpen?` true))))

(fn `UseItem`
  (params (ItemInfo :type "/Game/_BucolicAlone/Practice/PracticeBP/06_InventorySystem/Data/Structures/S_ItemStructure Structure"))
  (switch `/Game/_BucolicAlone/Practice/PracticeBP/06_InventorySystem/Data/Enums/E_ItemType` (`.Itemtype_6_B96ED54C48841BC72917508808F6824C` (break `/Game/_BucolicAlone/Practice/PracticeBP/06_InventorySystem/Data/Structures/S_ItemStructure` ItemInfo))
    (:`NewEnumerator0`
      (`self.ConsumeItem` ItemInfo))
    (:`NewEnumerator1`
      (`self.EquipItem` ItemInfo))
    (:`NewEnumerator2`
      (`self.ReadItem` ItemInfo))))

(fn `UserConstructionScript`)