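; BP_HealBox is a practice healing volume that restores the player character's health while it stays inside the box.
; On overlap with BP_Prac_PlayerCharacter, it stores the character and starts a looping one-second timer that clears on end overlap.
; Each tick of the timer adds a fixed amount to Health, or prints a message instead when Health exactly equals the maximum, with no clamping.
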(event `self.BoxCollision.OnComponentBeginOverlap`
  (params (OverlappedComponent :type "PrimitiveComponent Object Reference") (OtherActor :type "Actor Object Reference") (OtherComp :type "PrimitiveComponent Object Reference") (OtherBodyIndex :type Integer) (bFromSweep :type Boolean) (SweepResult :type "HitResult Structure (by ref)"))
  (bind _asbp_prac_player_character (cast `/Game/_BucolicAlone/Practice/Blueprints/BP_Prac_PlayerCharacter` OtherActor))
  (set `self.As BP Prac Player Character` _asbp_prac_player_character)
  (bind _returnvalue (`KismetSystemLibrary.K2_SetTimerDelegate` (delegate `HealPlayer`) 1.0 true))
  (set `self.TimerReference` _returnvalue))

(event `HealPlayer`
  (bind _as_bp_prac_player_character (`self.As BP Prac Player Character`))
  (if (== (`/Game/_BucolicAlone/Practice/Blueprints/BP_Prac_PlayerCharacter.Health` (`self.As BP Prac Player Character`)) 100.0)
    (`KismetSystemLibrary.PrintString` "Health is already cured")
    (else
      (set `/Game/_BucolicAlone/Practice/Blueprints/BP_Prac_PlayerCharacter.Health` (+ (`/Game/_BucolicAlone/Practice/Blueprints/BP_Prac_PlayerCharacter.Health` _as_bp_prac_player_character) 10.0) _as_bp_prac_player_character))))

(event `self.BoxCollision.OnComponentEndOverlap`
  (params (OverlappedComponent :type "PrimitiveComponent Object Reference") (OtherActor :type "Actor Object Reference") (OtherComp :type "PrimitiveComponent Object Reference") (OtherBodyIndex :type Integer))
  (cast `/Game/_BucolicAlone/Practice/Blueprints/BP_Prac_PlayerCharacter` OtherActor)
  (`KismetSystemLibrary.K2_ClearAndInvalidateTimerHandle` (`self.TimerReference`)))

(fn `UserConstructionScript`)