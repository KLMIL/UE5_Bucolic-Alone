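; BP_SoccerGoal is a soccer practice goal that detects a ball entering it and respawns a new one.
; On BeginPlay it caches the location of the referenced ball, if valid, as the spawn point.
; When a BP_SoccerBall overlaps BoxCollision, it plays a hit particle effect above the goal and destroys the ball.
; After a short delay it spawns a fresh ball at the cached location.
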(event `self.BoxCollision.OnComponentBeginOverlap`
  (params (OverlappedComponent :type "PrimitiveComponent Object Reference") (OtherActor :type "Actor Object Reference") (OtherComp :type "PrimitiveComponent Object Reference") (OtherBodyIndex :type Integer) (bFromSweep :type Boolean) (SweepResult :type "HitResult Structure (by ref)"))
  (bind _asbp_soccer_ball (cast `/Game/_BucolicAlone/Practice/PracticeBP/04_SoccerGame/Blueprints/BP_SoccerBall` OtherActor))
  (`GameplayStatics.SpawnEmitterAtLocation` "/Game/_BucolicAlone/Practice/PracticeBP/04_SoccerGame/Particles/P_Prac_ky_hit1.P_Prac_ky_hit1" (`KismetMathLibrary.MakeVector` (.x (`self.K2_GetActorLocation`)) (.y (`self.K2_GetActorLocation`)) (+ (.z (`self.K2_GetActorLocation`)) 300.0)) (struct) (2.0 2.0 2.0))
  (`self.K2_DestroyActor` _asbp_soccer_ball)
  (`KismetSystemLibrary.Delay` 1.0)
  (`|SpawnActorFromClass` "/Game/_BucolicAlone/Practice/PracticeBP/04_SoccerGame/Blueprints/BP_SoccerBall.BP_SoccerBall_C" (`KismetMathLibrary.MakeTransform` (stale `self.ReceiveBeginPlay` _output_get)) "Undefined" "MultiplyWithRoot" null null))

(event `self.ReceiveBeginPlay`
  (bind _soccerballreference (`self.SoccerBallReference`))
  (`/Engine/EditorBlueprintResources/StandardMacros.IsValid` _soccerballreference
    (:`Is Valid`
      (bind _output_get (set `self.SpawnSoccerBallLocation` (`self.K2_GetActorLocation` _soccerballreference))))))

(fn `UserConstructionScript`)